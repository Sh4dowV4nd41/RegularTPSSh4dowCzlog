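; Pickup weapon actor that the player can equip, drop, holster and switch between on the ThirdPersonCharacter.
; Overlapping its collision enables input; leaving disables it while the character is unarmed.
; Equip holsters the current weapon, drops any sharing its secondary socket, then snaps itself to the primary socket, yet sets IsArmedBP false.
; Select picks long or short weapons by fixed attached-actor index and sets IsArmedBP true; Next alternates between them.
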(event OnComponentBeginOverlap(Collision)
  (params (OverlappedComponent :type Primitive%20Component%20Object%20Reference) (OtherActor :type Actor%20Object%20Reference) (OtherComp :type Primitive%20Component%20Object%20Reference) (OtherBodyIndex :type Integer) (bFromSweep :type Boolean) (SweepResult :type Hit%20Result%20Structure%20%28by%20ref%29))
  (CallFunction|InputEnable true))

(event OnComponentEndOverlap(Collision)
  (params (OverlappedComponent :type Primitive%20Component%20Object%20Reference) (OtherActor :type Actor%20Object%20Reference) (OtherComp :type Primitive%20Component%20Object%20Reference) (OtherBodyIndex :type Integer))
  (bind _asthird_person_character (Utilities|Casting|CastToThirdPersonCharacter (Game|GetPlayerCharacter 0)))
  (if (not (Variables|/Game/ThirdPersonBP/Blueprints/ThirdPersonCharacter.ThirdPersonCharacter_C|GetIsArmed_BP _asthird_person_character))
    (CallFunction|InputEnable false)))

(event EventBeginPlay)

(event Collision|EventActorBeginOverlap
  (params (OtherActor :type Actor%20Object%20Reference)))

(event EventTick
  (params (DeltaSeconds :type Float%20%28single-precision%29)))

(event Input|ActionEvents|InputActionEquip
  (params (Key :type Key%20Structure))
  (:Pressed
    (CallFunction|Equip)))

(event Input|ActionEvents|InputActionDesequip
  (params (Key :type Key%20Structure))
  (:Pressed
    (CallFunction|Desequip)))

(event Input|ActionEvents|InputActionKeep
  (params (Key :type Key%20Structure))
  (:Pressed
    (CallFunction|Keep)))

(event Input|ActionEvents|InputActionLongWeapon
  (params (Key :type Key%20Structure))
  ;[1 1 1] Select Weapon
  (:Pressed
    (CallFunction|Select "Long")))

(event Input|ActionEvents|InputActionShortWeapon
  (params (Key :type Key%20Structure))
  ;[1 1 1] Select Weapon
  (:Pressed
    (CallFunction|Select "Short")))

(event Input|ActionEvents|InputActionNext
  (params (Key :type Key%20Structure))
  ;[1 1 1] Select Weapon
  (:Pressed
    (Utilities|FlowControl|FlipFlop
      (:A
        (CallFunction|Select "Long"))
      (:B
        (CallFunction|Select "Short")))))

(fn ConstructionScript)

(fn Equip
  (CallFunction|Keep)
  (bind _asthird_person_character (Utilities|Casting|CastToThirdPersonCharacter (Game|GetPlayerCharacter 0)))
  (bind _output_get (LocalVariables|SetTPC _asthird_person_character))
  (for _array_element (Actor|GetAttachedActors _output_get)
    (bind _asweapon_bp (Utilities|Casting|CastToWeapon_BP _array_element))
    (if (Utilities|Name|Equal(Name) (Variables|Weapon_BP_C|GetSecondarySocket _asweapon_bp) (Variables|Default|GetSecondarySocket))
      (CallFunction|Desequip _asweapon_bp)))
  (Transformation|AttachComponentToComponent self (Variables|/Script/Engine.Character|GetMesh (LocalVariables|GetTPC)) (Variables|Default|GetPrimarySocket) "SnapToTarget" "SnapToTarget" "SnapToTarget" true)
  (Variables|/Game/ThirdPersonBP/Blueprints/ThirdPersonCharacter.ThirdPersonCharacter_C|SetIsArmed_BP (LocalVariables|GetTPC) false)
  (Variables|/Game/ThirdPersonBP/Blueprints/ThirdPersonCharacter.ThirdPersonCharacter_C|SetCurrentWeapon (LocalVariables|GetTPC) self)
  (Physics|SetSimulatePhysics (Variables|Default|GetWeapon) false))

(fn Desequip
  (params (Weapon :type Weapon%20BP%20Object%20Reference))
  (bind _asthird_person_character (Utilities|Casting|CastToThirdPersonCharacter (Game|GetPlayerCharacter 0)))
  (Variables|/Game/ThirdPersonBP/Blueprints/ThirdPersonCharacter.ThirdPersonCharacter_C|SetIsArmed_BP _asthird_person_character false)
  (Variables|/Game/ThirdPersonBP/Blueprints/ThirdPersonCharacter.ThirdPersonCharacter_C|SetCurrentWeapon _asthird_person_character 0)
  (Utilities|IsValid Weapon
    (:Is%20Valid
      (Transformation|DetachFromActor Weapon "KeepWorld" "KeepWorld" "KeepWorld"))
    (:Is%20Not%20Valid
      (Transformation|DetachFromActor "KeepWorld" "KeepWorld" "KeepWorld")))
  (Physics|SetSimulatePhysics (Variables|Default|GetWeapon) true))

(fn InputEnable
  (params (Enable :type Boolean))
  (bind _returnvalue (Game|GetPlayerController 0))
  ;[1 1 1] Act o Desact el uso de teclas al actor
  (if Enable
    (Input|EnableInput _returnvalue)
    (else
      (Input|DisableInput _returnvalue))))

(fn Keep
  (bind _returnvalue (Game|GetPlayerCharacter 0))
  (bind _asthird_person_character (Utilities|Casting|CastToThirdPersonCharacter _returnvalue))
  (Utilities|IsValid (Variables|/Game/ThirdPersonBP/Blueprints/ThirdPersonCharacter.ThirdPersonCharacter_C|GetCurrentWeapon _asthird_person_character)
    (:Is%20Valid
      (Transformation|AttachComponentToComponent (Variables|/Game/ThirdPersonBP/Blueprints/ThirdPersonCharacter.ThirdPersonCharacter_C|GetCurrentWeapon _asthird_person_character) (Variables|/Script/Engine.Character|GetMesh _returnvalue) (Variables|Weapon_BP_C|GetSecondarySocket (Variables|/Game/ThirdPersonBP/Blueprints/ThirdPersonCharacter.ThirdPersonCharacter_C|GetCurrentWeapon _asthird_person_character)) "SnapToTarget" "SnapToTarget" "SnapToTarget" true)
      (Variables|/Game/ThirdPersonBP/Blueprints/ThirdPersonCharacter.ThirdPersonCharacter_C|SetIsArmed_BP _asthird_person_character false)
      (Variables|/Game/ThirdPersonBP/Blueprints/ThirdPersonCharacter.ThirdPersonCharacter_C|SetCurrentWeapon _asthird_person_character 0))))

(fn Select
  (params (WeaponType :type String))
  (bind _returnvalue (Game|GetPlayerCharacter 0))
  (bind _primarysocket (Variables|Default|GetPrimarySocket))
  (CallFunction|Keep)
  (bind _asthird_person_character (Utilities|Casting|CastToThirdPersonCharacter _returnvalue))
  (LocalVariables|SetTPC _asthird_person_character)
  (LocalVariables|SetTPCMesh (Variables|/Script/Engine.Character|GetMesh _returnvalue))
  (if (Utilities|Enum|Equal(Enum) WeaponType "Long")
    (bind _asweapon_bp (Utilities|Casting|CastToWeapon_BP (Utilities|Array|Get(acopy) (Actor|GetAttachedActors (LocalVariables|GetTPC)) 1)))
    (Transformation|AttachComponentToComponent _asweapon_bp (LocalVariables|GetTPCMesh) _primarysocket "SnapToTarget" "SnapToTarget" "SnapToTarget" true)
    (Variables|/Game/ThirdPersonBP/Blueprints/ThirdPersonCharacter.ThirdPersonCharacter_C|SetCurrentWeapon (LocalVariables|GetTPC) _asweapon_bp)
    (else
      (bind _asweapon_bp_2 (Utilities|Casting|CastToWeapon_BP (Utilities|Array|Get(acopy) (Actor|GetAttachedActors (LocalVariables|GetTPC)))))
      (Transformation|AttachComponentToComponent _asweapon_bp_2 (LocalVariables|GetTPCMesh) _primarysocket "SnapToTarget" "SnapToTarget" "SnapToTarget" true)
      (Variables|/Game/ThirdPersonBP/Blueprints/ThirdPersonCharacter.ThirdPersonCharacter_C|SetCurrentWeapon (LocalVariables|GetTPC) _asweapon_bp_2)))
  (Variables|/Game/ThirdPersonBP/Blueprints/ThirdPersonCharacter.ThirdPersonCharacter_C|SetIsArmed_BP (LocalVariables|GetTPC) true))